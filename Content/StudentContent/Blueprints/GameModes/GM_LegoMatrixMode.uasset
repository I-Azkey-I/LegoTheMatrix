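; Game mode for a Lego Matrix game that sets up local multiplayer for up to two players on a shared camera.
; On BeginPlay it spawns a character per BP_PlayerSpawn, creates and initialises its controller, and blends to BP_MainCamera, warning instead if over two spawns exist.
; StartGame checks the minimum player count, enabling swapping and initiating the shared camera only when that minimum is one.
; SwapCharacter spawns replacement characters.
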(event `self.ReceiveBeginPlay`
  ;[1 1 1] Initialisation Chain (Game Mode Management)
  ;;[0.6795 1 0.5776] Find main shared camera in the scene.
  (bind _outactors (`GameplayStatics.GetAllActorsOfClass` "/Game/StudentContent/Blueprints/Actors/Cameras/BP_MainCamera.BP_MainCamera_C"))
  (set `self.Main Camera` (`|GetArrayItem` _outactors))
  ;;[0.6795 1 0.5776] Find all player spawn locations.
  (`self.Get Player Spawn Locals`)
  ;;[0.6795 1 0.5776] Spawn all initial player characters (ENSURE ONLY TWO ARE IN PLAY).
  (if (not (> (`KismetArrayLibrary.Array_Length` (`self.Player Spawn Locals`)) 2))
    (`self.Spawn Player Characters`)
    (else
      (`PlayerController.SetViewTargetWithBlend` (`GameplayStatics.GetPlayerController` 0) (`self.Main Camera`) 0.0 "VTBlend_Linear" 0.0 false)
      (`KismetSystemLibrary.PrintString` "Please use only TWO spawn locations for multi-player system!" true true (struct :`R` 1.0 :`A` 1.0) 6.0)
      (`KismetSystemLibrary.PrintString` "TWO PLAYERS ONLY!" true true (struct :`R` 1.0 :`A` 1.0) 6.0))))

(fn `Get Player Spawn Locals`
  ;[0.6795 1 0.5776] Find all player spawn locations in the scene.
  (bind _outactors (`GameplayStatics.GetAllActorsOfClass` "/Game/StudentContent/Blueprints/Actors/BP_PlayerSpawn.BP_PlayerSpawn_C"))
  (set `self.Player Spawn Locals` _outactors)
  (return))

(fn `Remove Unused Cameras`
  ;[0.6795 1 0.5776] Destroy all camera's (apart from main camera) in the scene.
  (bind _outactors (`GameplayStatics.GetAllActorsOfClass` "/Script/Engine.CameraActor"))
  (for _array_element _outactors
    (`self.K2_DestroyActor` _array_element)))

(fn `Spawn Player Character (Basic)`
  (params (`Character Index` :type Integer) (`Transform Data` :type "Transform Structure"))
  (returns (ReturnValue :type "/Game/StudentContent/Blueprints/Actors/Pawns/Characters/Players/BPC_BasePlayer Object Reference"))
  (bind _output (`|GetArrayItem` (`self.Swappable Characters`) `Character Index`))
  ;[0.6795 1 0.5776] Select from list of available characters (using character index) to spawn into the scene.
  (bind _returnvalue (`|SpawnActorFromClass` (select `int` `Character Index` :`0` _output :`1` _output) (`KismetMathLibrary.MakeTransform` (.location `Transform Data`) (struct) (.scale `Transform Data`)) "Undefined" "OverrideRootScale" null `Character Index` null))
  (return _returnvalue))

(fn `Spawn Player Characters`
  (locals (`Spawn Location Index (L)` :type Integer))
  (bind _player_controllers (`self.Player Controllers`))
  (bind _returnvalue (`GameplayStatics.GetPlayerController` (`self.Player Spawn ID`)))
  ;[1 1 1] Player Spawning Management (New Scenes)
  ;;[0.6795 1 0.5776] For each spawn location, store their index & ID, then create their respective player controller.
  (for (_array_element _array_index) (`self.Player Spawn Locals`)
    (set `local.Spawn Location Index (L)` _array_index)
    (bind _output_get (set `self.Player Spawn ID` (`/Game/StudentContent/Blueprints/Actors/BP_PlayerSpawn.PlayerSpawnID` _array_element)))
    (`GameplayStatics.CreatePlayer` _output_get)
    ;;[0.6795 1 0.5776] Spawn a character at each spawn location (based on local index).
    (bind _spawned_character (`self.Spawn Players` (`self.Player Spawn ID`) (`self.GetTransform` (`|GetArrayItem` (`self.Player Spawn Locals`) (`local.Spawn Location Index (L)`)))))
    ;;[0.6795 1 0.5776] Possess each player character with the relevant player controller.
    (`Controller.Possess` _returnvalue _spawned_character)
    (bind _returnvalue_2 (`KismetArrayLibrary.Array_AddUnique` _player_controllers _returnvalue))
    ;;[0.6795 1 0.5776] Initialise the player controllers for each player character.
    (message `/Game/StudentContent/Blueprints/Libraries/BPI_MatrixMode.Initialise Controller` (`|GetArrayItem` _player_controllers _returnvalue_2))
    ;;[0.6795 1 0.5776] Blend the camera of each controller to the main shared camera.
    (`PlayerController.SetViewTargetWithBlend` (`GameplayStatics.GetPlayerController` (`self.Player Spawn ID`)) (`self.Main Camera`) 0.0 "VTBlend_Linear" 0.0 false))
  ;;[0.6795 1 0.5776] Once all characters have spawned, remove all other cameras & initialise other game features.
  (`self.Remove Unused Cameras`)
  (`self.Start Game`)
  ;;[0.6795 1 0.5776] Assign each player controller an array of current characters (for main camera updates).
  (for _array_element_2 (`self.Player Controllers`)
    (bind _asbp_player_controller (cast `/Game/StudentContent/Blueprints/Actors/Pawns/Characters/Players/BP_PlayerController` _array_element_2))
    (`KismetArrayLibrary.Array_Append` (`/Game/StudentContent/Blueprints/Actors/Pawns/Characters/Players/BP_PlayerController.Current Characters` _asbp_player_controller) (`self.Spawned Characters`))))

(fn `Spawn Players`
  (params (`Character Spawn Index` :type Integer) (`Transform Data` :type "Transform Structure"))
  (returns (`Spawned Character` :type "/Game/StudentContent/Blueprints/Actors/Pawns/Characters/Players/BPC_BasePlayer Object Reference"))
  ;[0.6795 1 0.5776] Spawn a player character into a new scene at an assigned location.
  (bind _output_get (set `self.Character Spawn Index` `Character Spawn Index`))
  (bind _returnvalue (`self.Spawn Player Character (Basic)` _output_get `Transform Data`))
  (`KismetArrayLibrary.Array_Add` (`self.Spawned Characters`) _returnvalue)
  (return _returnvalue))

(fn `Start Game`
  (returns (Return :type Boolean))
  ;[1 1 1] Initial "Start Game" Behaviour / Conditions
  ;;[0.6795 1 0.5776] Begin the game when min. number of players has been reached.
  (if (>= (`KismetArrayLibrary.Array_Length` (`self.Spawned Characters`)) (`self.Min Number of Players`))
    (set `self.Has Game Started?` true)
    ;;[0.6795 1 0.5776] If the min. number of players is = 1, allow this player to swap between characters.
    (if (== (`self.Min Number of Players`) 1)
      (set `self.Player Can Swap` true)
      ;;[0.6795 1 0.5776] Instantiate the shared camera for all readied players.
      (`/Game/StudentContent/Blueprints/Actors/Cameras/BP_MainCamera.Initiate Shared Camera` (`self.Main Camera`) (`self.Spawned Characters`))
      (return false))))

(fn `Swap Character`
  (params (`Character Index` :type Integer) (`Transform Data` :type "Transform Structure"))
  (returns (`New Player Character` :type "/Game/StudentContent/Blueprints/Actors/Pawns/Characters/BP_BaseCharacter Object Reference"))
  ;[0.6795 1 0.5776] Spawn a new character into scene to be swapped with old character.
  (bind _returnvalue (`self.Spawn Player Character (Basic)` `Character Index` `Transform Data`))
  (return _returnvalue))

(fn `UserConstructionScript`)
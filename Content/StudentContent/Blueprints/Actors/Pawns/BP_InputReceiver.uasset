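; BP_InputReceiver is a per-player input pawn that lets a player request a character spawn while the game is not in play.
; On BeginPlay it finds and stores BP_GameManager.
; Pressing Spawn checks the manager's play state via an interface message, then passes it the receiver's index and itself to spawn, printing a confirmation.
; Its own play-state, spawn, start and swap functions are empty stubs.
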(event `self.ReceiveBeginPlay`
  ;[0.6795 1 0.5776] Find the "Game Manager" in the scene.
  (bind _returnvalue (`GameplayStatics.GetActorOfClass` "/Game/StudentContent/Blueprints/Managers/BP_GameManager.BP_GameManager_C"))
  (set `self.Game Manager (Ref)` _returnvalue))

(event `InputAction|Spawn`
  (params (Key :type "Key Structure"))
  (bind _input_receiver_index (`self.Input Receiver Index`))
  ;[1 1 1] Spawn Input Receivers
  ;;[0.6795 1 0.5776] Check to the game's current play state.
  (:`Pressed`
    (bind _in_play_state (message `/Game/StudentContent/Blueprints/Libraries/BPI_StartGame.Is In Play State?` (`self.Game Manager (Ref)`)))
    (if (not _in_play_state)
      ;;[0.6795 1 0.5776] If not in player state, allow the spawning of player characters.
      (message `/Game/StudentContent/Blueprints/Libraries/BPI_StartGame.Spawn Player` (`self.Game Manager (Ref)`) _input_receiver_index self)
      (`KismetSystemLibrary.PrintString` (`KismetStringLibrary.Concat_StrStr` "Player " (`KismetStringLibrary.Conv_IntToString` (+ _input_receiver_index 1)) " has spawned!") true true (struct :`R` 0.079539 :`G` 1.0 :`A` 1.0)))))

(fn `Is In Play State?`
  (returns (`In Play State` :type Boolean))
  (return false))

(fn `Spawn Player`
  (params (`Current Player Index` :type Integer) (`Input Receiver` :type "/Game/StudentContent/Blueprints/Actors/Pawns/BP_InputReceiver Object Reference"))
  (returns (Return :type Boolean))
  (return false))

(fn `Start Game`
  (returns (Return :type Boolean))
  (return false))

(fn `Swap Character`
  (params (`Character Index` :type Integer) (`Transform Data` :type "Transform Structure"))
  (returns (`New Player Character` :type "/Game/StudentContent/Blueprints/Actors/Pawns/Characters/BP_BaseCharacter Object Reference") (Return :type Boolean))
  (return null false))

(fn `UserConstructionScript`)
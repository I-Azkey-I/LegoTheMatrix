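; Player controller for the Lego Matrix game mode that swaps the player's character on the Character Swap input.
; It loops over the mode's swappable classes, respawning at the current transform for every class differing from the initially possessed one.
; Each respawn destroys the old pawn, has the game mode supply the new one, possesses it and updates the shared camera.
; Score, damage and health events are empty, with their stat logic left unconnected.
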(event `/Game/StudentContent/Blueprints/Libraries/BPI_CharacterStats.Add Score`
  (params (Score :type Integer))
  ;[1 1 1] Player Stats
  ;;[0.6795 1 0.5776] Add score to player (Interface Event).
)

(event `/Game/StudentContent/Blueprints/Libraries/BPI_CharacterStats.Apply Damage`
  (params (Damage :type "Float (single-precision)"))
  ;[1 1 1] Player Stats
  ;;[0.6795 1 0.5776] Apply damage to the player (Interface Event).
)

(event `/Game/StudentContent/Blueprints/Libraries/BPI_CharacterStats.Increase Health`
  (params (`Add. Health` :type "Float (single-precision)"))
  ;[1 1 1] Player Stats
  ;;[0.6795 1 0.5776] Apply health to the player (Interface Event).
)

(event `/Game/StudentContent/Blueprints/Libraries/BPI_MatrixMode.Initialise Controller`
  ;[1 1 1] Initial Behaviour
  ;;[0.6795 1 0.5776] Pass through any and all relevant variables for use in this blueprint (Interface Event).
  (bind _asgm_lego_matrix_mode (cast `/Game/StudentContent/Blueprints/GameModes/GM_LegoMatrixMode` (`GameplayStatics.GetGameMode`)))
  (set `self.Main Camera` (`/Game/StudentContent/Blueprints/GameModes/GM_LegoMatrixMode.Main Camera` _asgm_lego_matrix_mode))
  (set `self.Swappable Characters` (`/Game/StudentContent/Blueprints/GameModes/GM_LegoMatrixMode.Swappable Characters` _asgm_lego_matrix_mode)))

(event `InputAction|Character Swap`
  (params (Key :type "Key Structure"))
  (bind _returnvalue (`self.Retrieve Character`))
  ;[1 1 1] Character Swapping System
  ;;[0.6795 1 0.5776] Find the current possessed character class.
  (:`Pressed`
    (set `self.Possessed Character Class` (`self.Retrieve Character Class`))
    ;;[0.6795 1 0.5776] Compare possessed character with available swappable characters.
    (for (_array_element _array_index) (`self.Swappable Characters`)
      (set `self.Swappable Character Index` _array_index)
      (if (not (== _array_element (`self.Possessed Character Class`)))
        ;;[0.6795 1 0.5776] If characters are different, store relevant data of current possessed character.
        (set `self.Character Transform Data` (`self.GetTransform` _returnvalue))
        ;;[0.6795 1 0.5776] Respawn the player character into the scene.
        (`self.Respawn Player Character` (`self.Swappable Character Index`) (`self.Character Transform Data`) _returnvalue)))))

(fn `Respawn Player Character`
  (params (`Character Index` :type Integer) (`Transform Data` :type "Transform Structure") (`Current Character` :type "Character Object Reference"))
  (bind _main_camera (`self.Main Camera`))
  ;[0.6795 1 0.5776] Unpossess and remove the old character.
  (`self.UnPossess`)
  (`KismetArrayLibrary.Array_RemoveItem` (`self.Current Characters`) `Current Character`)
  (`self.K2_DestroyActor` `Current Character`)
  ;[0.6795 1 0.5776] Spawn the new character, update the "Current Characters" array and possess them.
  (bind _new_player_character (message `/Game/StudentContent/Blueprints/Libraries/BPI_MatrixMode.Swap Character` (`GameplayStatics.GetGameMode`) `Character Index` `Transform Data`))
  (`KismetArrayLibrary.Array_Add` (`self.Current Characters`) _new_player_character)
  (`self.Possess` _new_player_character)
  ;[0.6795 1 0.5776] Update all camera information & functionality.
  (`/Game/StudentContent/Blueprints/Actors/Cameras/BP_MainCamera.Update Shared Camera` _main_camera (`self.Current Characters`))
  (`self.SetViewTargetWithBlend` _main_camera))

(fn `Retrieve Character`
  (returns (ReturnValue :type "Character Object Reference"))
  ;[0.6795 1 0.5776] Return the character actor.
  (return (`GameplayStatics.GetPlayerCharacter` (`GameplayStatics.GetPlayerControllerID` self))))

(fn `Retrieve Character Class`
  (returns (ReturnValue :type "Character Class Reference"))
  ;[0.6795 1 0.5776] Return the character class.
  (return (`GameplayStatics.GetObjectClass` (`GameplayStatics.GetPlayerCharacter` (`GameplayStatics.GetPlayerControllerID` self)))))

(fn `Start Game`
  (returns (Return :type Boolean))
  (return false))

(fn `Swap Character`
  (params (`Character Index` :type Integer) (`Transform Data` :type "Transform Structure"))
  (returns (`New Player Character` :type "/Game/StudentContent/Blueprints/Actors/Pawns/Characters/BP_BaseCharacter Object Reference"))
  (return null))

(fn `UserConstructionScript`)
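; AI controller for patrolling enemies that chase and attack players, driven by the BT_NewEnemyAI behavior tree.
; On possess it runs the tree and seeds patrol blackboard keys from the enemy's patrol path.
; Perception updates are handled by stimulus index: seeing a tagged player or being hit sets the chase keys, with hits reusing the last seen actor.
; Failed stimuli start a line-of-sight timer, with SetEnemyTimer providing the chase-key reset.
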(event `self.ReceivePossess`
  (params (PossessedPawn :type "Pawn Object Reference"))
  (bind _returnvalue (`AIBlueprintHelperLibrary.GetBlackboard` null))
  ;[1 1 1] Enemy Patrol & Chase System
  ;;[0.6795 1 0.5776] Run the enemy's behaviour tree.).
  (`self.RunBehaviorTree` "/Game/StudentContent/Blueprints/Actors/Pawns/Characters/Enemies/BT_NewEnemyAI.BT_NewEnemyAI")
  ;;[0.6795 1 0.5776] Store reference to possessed enemy character.
  (bind _asbpc_enemy_character (cast `/Game/StudentContent/Blueprints/Actors/Pawns/Characters/Enemies/BPC_EnemyCharacter` (`self.K2_GetPawn`)))
  (set `self.Enemy Character (Ref)` _asbpc_enemy_character)
  ;;[0.6795 1 0.5776] Initial values to be set (after behaviour tree initialisation).
  (`BlackboardComponent.SetValueAsBool` _returnvalue "Is Looping" (`/Game/StudentContent/Blueprints/Actors/Pawns/Characters/Enemies/BP_PatrolPath.Is Looping` (`/Game/StudentContent/Blueprints/Actors/Pawns/Characters/Enemies/BPC_EnemyCharacter.Patrol Path (Ref)` (`self.Enemy Character (Ref)`))))
  (`BlackboardComponent.SetValueAsInt` _returnvalue "Path Direction" 1))

(event `self.AIPerception.OnPerceptionUpdated`
  (params (UpdatedActors :type "Array of Actor Object Reference (by ref)"))
  ;[1 1 1] Enemy Patrol & Chase System
  ;;[0.6795 1 0.5776] AI Perception Behaviour (React to Stimuli)
  (for _array_element UpdatedActors
    (bind _info (`AIPerceptionComponent.GetActorsPerception` (`self.AIPerception`) _array_element))
    (`self.Completed Senses` _array_element (`.LastSensedStimuli` (break `ActorPerceptionBlueprintInfo` _info)))))

(fn `Completed Senses`
  (params (`AI Actors` :type "Actor Object Reference") (Array :type "Array of AIStimulus Structure"))
  (locals (`AI Senses (L)` :type "AIStimulus Structure"))
  (bind _blackboard (`self.Blackboard`))
  (bind (_ai_senses__l__age _ai_senses__l__expirationage _ai_senses__l__strength _ai_senses__l__stimuluslocation _ai_senses__l__receiverlocation _ai_senses__l__tag _ai_senses__l__bsuccessfullysensed) (break `AIStimulus` (`local.AI Senses (L)`)))
  (bind _blackboard_2 (`self.Blackboard`))
  (bind (_ai_senses__l__age_2 _ai_senses__l__expirationage_2 _ai_senses__l__strength_2 _ai_senses__l__stimuluslocation_2 _ai_senses__l__receiverlocation_2 _ai_senses__l__tag_2 _ai_senses__l__bsuccessfullysensed_2) (break `AIStimulus` (`local.AI Senses (L)`)))
  ;[1 1 1] AI Controller Tasks with Behaviour Tree
  ;;[0.6795 1 0.5776] For each AI Perception for each actor, execute a specific action / behaviour.
  (for (_array_element _array_index) Array
    (set `local.AI Senses (L)` _array_element)
    (switch `int` _array_index
      (:`0`
        ;;[0.6795 1 0.5776] When AI "SEES" a player, execute "Chase & Attacking" Behaviour of Behaviour Tree
        (if (and _ai_senses__l__bsuccessfullysensed_2 (`self.ActorHasTag` `AI Actors` "Players"))
          (set `self.Seen Actor` `AI Actors`)
          (`KismetSystemLibrary.K2_ClearAndInvalidateTimerHandle` (`self.Enemy Chase Timer`))
          (`BlackboardComponent.SetValueAsBool` _blackboard_2 "Has Seen Player" _ai_senses__l__bsuccessfullysensed_2)
          (`BlackboardComponent.SetValueAsObject` _blackboard_2 "Players" (`self.Seen Actor`))
          (else
            (bind _returnvalue (`KismetSystemLibrary.K2_SetTimerDelegate` (`|CreateDelegate` :!event `Set Enemy Timer`) (`self.Line of Sight Time`)))
            (set `self.Enemy Chase Timer` _returnvalue))))
      (:`2`
        ;;[0.6795 1 0.5776] When AI is "HIT" by player, execute "Chasing & Attacking" Behaviour of Behaviour Tree
        (if _ai_senses__l__bsuccessfullysensed
          (`BlackboardComponent.SetValueAsBool` _blackboard "Has Seen Player" _ai_senses__l__bsuccessfullysensed)
          (`BlackboardComponent.SetValueAsObject` _blackboard "Players" (`self.Seen Actor`))
          (else
            (bind _returnvalue_2 (`KismetSystemLibrary.K2_SetTimerDelegate` (`|CreateDelegate` :!event `Set Enemy Timer`) (`self.Line of Sight Time`)))
            (set `self.Enemy Chase Timer` _returnvalue_2)))))))

(fn `Set Enemy Timer`
  (bind _blackboard (`self.Blackboard`))
  ;[0.6795 1 0.5776] Reset blackboard key values when AI looses sight of player(s).
  (`BlackboardComponent.SetValueAsBool` _blackboard "Has Seen Player" false)
  (`BlackboardComponent.SetValueAsObject` _blackboard "Players" null))

(fn `UserConstructionScript`)
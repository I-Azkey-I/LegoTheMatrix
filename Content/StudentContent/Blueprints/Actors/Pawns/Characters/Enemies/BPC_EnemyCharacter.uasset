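; Enemy character that punches with a melee attack, takes damage and is destroyed when its health runs out.
; MeleeAttack plays a punch montage whose notify sphere-traces forward from the right-hand socket to apply damage, with persistent debug drawing.
; Incoming damage reduces Health in the CharacterStats struct before the death check.
; The construction script tints guard enemies red and others pink, and a helper function sets walk speed.
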(event `self.ReceiveBeginPlay`
  ;[1 1 1] Enemy Character(s) Behaviour
  ;;[0.6795 1 0.5776] Initialise character stats relevant to enemies.
  (`parent.ReceiveBeginPlay`))

(event `/Game/StudentContent/Blueprints/Libraries/BPI_EnemyCombat.MeleeAttack`
  (bind _returnvalue (`SceneComponent.GetSocketLocation` (`self.Mesh`) "SOK_RightHand"))
  ;[1 1 1] Enemy Character(s) Behaviour
  ;;[0.6795 1 0.5776] Perform a melee attack with this event is called.
  (`|PlayMontage` (`self.Mesh`) "/Game/StudentContent/Blueprints/Actors/Pawns/Characters/Animations/AnimMon_Punch01.AnimMon_Punch01"
    (:`OnNotifyBegin`
      (bind _outhit (`KismetSystemLibrary.SphereTraceSingle` :`Start` _returnvalue :`End` (+ _returnvalue (* (`KismetMathLibrary.GetForwardVector` (`self.K2_GetActorRotation`)) 75.0)) :`Radius` 50.0 :`TraceChannel` "TraceTypeQuery2" :`DrawDebugType` "Persistent"))
      ;;[0.6795 1 0.5776] If enemy hits a player character, apply a small amount of damage.
      (if (== (`GameplayStatics.BreakHitResult` _outhit) (`KismetSystemLibrary.IsValid` (`.HitActor` (`GameplayStatics.BreakHitResult` _outhit))))
        (`GameplayStatics.ApplyDamage` (`.HitActor` (`GameplayStatics.BreakHitResult` _outhit)) 10.0 null null "/Script/Engine.DamageType")))))

(event `self.ReceiveAnyDamage`
  (params (Damage :type "Float (single-precision)") (DamageType :type "DamageType Object Reference") (InstigatedBy :type "Controller Object Reference") (DamageCauser :type "Actor Object Reference"))
  (bind (_character_stats_score _character_stats_health) (break `/Game/StudentContent/Blueprints/Actors/Pawns/Characters/Struct_CharacterStats` (`self.Character Stats`)))
  (setmembers `/Game/StudentContent/Blueprints/Actors/Pawns/Characters/Struct_CharacterStats` :`StructRef` (`self.Character Stats`) :`Health` (- _character_stats_health Damage))
  (`self.Character Dead?`))

(event `self.Character Dead?`
  (bind (_character_stats_score _character_stats_health) (break `/Game/StudentContent/Blueprints/Actors/Pawns/Characters/Struct_CharacterStats` (`self.Character Stats`)))
  (if (<= _character_stats_health 0.0)
    (`self.K2_DestroyActor`)))

(fn `Update Walk Speed`
  (params (`New Walking Speed` :type "Float (double-precision)"))
  ;[0.6795 1 0.5776] Update the enemy walking speed.
  (set `CharacterMovementComponent.MaxWalkSpeed` `New Walking Speed` (`self.CharacterMovement`)))

(fn `UserConstructionScript`
  (bind _mesh (`self.Mesh`))
  (bind _mesh_2 (`self.Mesh`))
  (if (`self.Is Guard Enemy`)
    (for (_ _array_index) (`MeshComponent.GetMaterials` _mesh_2)
      (`PrimitiveComponent.SetMaterial` _mesh_2 _array_index "/Game/StudentContent/Materials/Characters/TEMP_MATERIALS/MIns_Red.MIns_Red"))
    (else
      (for (_ _array_index_2) (`MeshComponent.GetMaterials` _mesh)
        (`PrimitiveComponent.SetMaterial` _mesh _array_index_2 "/Game/StudentContent/Materials/Characters/TEMP_MATERIALS/MIns_Pink.MIns_Pink")))))
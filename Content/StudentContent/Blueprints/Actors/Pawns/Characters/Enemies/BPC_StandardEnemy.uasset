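; BPC_StandardEnemy is an enemy character Blueprint with a melee punch attack and an adjustable walking speed.
; The MeleeAttack event plays a punch montage, whose notify triggers a forward sphere trace from the right-hand socket on the Camera channel.
; The trace draws persistent debug shapes, and its result is not used, so no damage is applied here.
; UpdateWalkSpeed sets the character movement's max walk speed.
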(event `/Game/StudentContent/Blueprints/Libraries/BPI_EnemyCombat.MeleeAttack`
  (bind _returnvalue (`SceneComponent.GetSocketLocation` (`self.Mesh`) "SOK_RightHand"))
  (`|PlayMontage` (`self.Mesh`) "/Game/StudentContent/Blueprints/Actors/Pawns/Characters/Animations/AnimMon_Punch01.AnimMon_Punch01"
    (:`OnNotifyBegin`
      (`KismetSystemLibrary.SphereTraceSingle` :`Start` _returnvalue :`End` (+ _returnvalue (* (`KismetMathLibrary.GetForwardVector` (`self.K2_GetActorRotation`)) 75.0)) :`Radius` 50.0 :`TraceChannel` "TraceTypeQuery2" :`DrawDebugType` "Persistent"))))

(fn `Update Walk Speed`
  (params (`New Walking Speed` :type "Float (double-precision)"))
  ;[0.6795 1 0.5776] Update the enemy walking speed.
  (set `CharacterMovementComponent.MaxWalkSpeed` `New Walking Speed` (`self.CharacterMovement`)))

(fn `UserConstructionScript`
  (`parent.UserConstructionScript`))
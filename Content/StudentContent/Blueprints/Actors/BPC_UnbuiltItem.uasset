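; Unbuilt item actor that players build by holding interact, a work-in-progress timed building mechanic.
; Its Interact Effect override starts a looping one-second timer on the first hold, pauses it on release and resumes it on later holds, so progress persists.
; Each tick decrements TimeValue and prints it, or a built message at zero; the timer is never cleared and no built result follows yet.
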(fn `Decrement Time`
  (bind _time_value (`self.Time Value`))
  ;[0.6795 1 0.5776] Decrement a value for the timer to fire off as a delegate.
  (set `self.Time Value` (- (`self.Time Value`) 1))
  (if (<= _time_value 0)
    (`KismetSystemLibrary.PrintString` "Item is built!")
    (else
      (`KismetSystemLibrary.PrintString` (`KismetStringLibrary.Conv_IntToString` _time_value)))))

(fn `Interact Effect`
  (params (`Player Character` :type "/Game/StudentContent/Blueprints/Actors/Pawns/Characters/BP_BaseCharacter Object Reference") (`Character Index` :type Integer) (`Holding Interact` :type Boolean))
  ;[1 0.5711 0] Timer for Building Items Mechanic (WORK IN PROGRESS)
  (if `Holding Interact`
    (if (`self.Partially Built`)
      (`KismetSystemLibrary.K2_UnPauseTimer` null "Decrement Time")
      (else
        (set `self.Partially Built` true)
        (bind _returnvalue (`KismetSystemLibrary.K2_SetTimer` null "Decrement Time" 1.0 true))
        (set `self.Timer Handle` _returnvalue)))
    (else
      (`KismetSystemLibrary.K2_PauseTimerHandle` (`self.Timer Handle`)))))

(fn `UserConstructionScript`
  (`parent.UserConstructionScript`))
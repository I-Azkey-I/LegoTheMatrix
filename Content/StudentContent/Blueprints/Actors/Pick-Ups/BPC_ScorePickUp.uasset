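; Score pick-up Blueprint for a stud collectible that awards points to the player who collects it.
; The construction script compares AddScore with the StudValues tiers and applies the matching silver, gold, blue or purple material to both stud meshes.
; PickUpEffect passes AddScore to the supplied player controller through AddScoreMessage.
; Both graphs are marked as testing-purpose implementations.
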(fn `Pick-Up Effect`
  (params (`Player Controller` :type "/Game/StudentContent/Blueprints/Actors/Pawns/Characters/Players/BP_PlayerController Object Reference"))
  ;[1 0.5711 0] Add applied score to relevant player (TESTING PURPOSES).
  (message `/Game/StudentContent/Blueprints/Libraries/BPI_CharacterStats.Add Score` `Player Controller` (`self.Add Score`)))

(fn `UserConstructionScript`
  (bind _add_score (`self.Add Score`))
  (bind (_silver _gold _blue _purple) (break `/Game/StudentContent/Blueprints/Actors/Pick-Ups/Struct_StudValues` (`self.Stud Values`)))
  ;[1 0.9106 0.4452] Change stud colour based on score value (TESTING PURPOSES).
  (if (== _add_score _silver)
    (`PrimitiveComponent.SetMaterial` (`self.SM_Stud_1`) 0 "/Game/StudentContent/Materials/Pick-Ups/TEMP_MATERIALS/M_Silver.M_Silver")
    (`PrimitiveComponent.SetMaterial` (`self.SM_Stud_2`) 0 "/Game/StudentContent/Materials/Pick-Ups/TEMP_MATERIALS/M_Silver.M_Silver")
    (elif (== _add_score _gold)
      (`PrimitiveComponent.SetMaterial` (`self.SM_Stud_1`) 0 "/Game/StudentContent/Materials/Pick-Ups/TEMP_MATERIALS/M_Gold.M_Gold")
      (`PrimitiveComponent.SetMaterial` (`self.SM_Stud_2`) 0 "/Game/StudentContent/Materials/Pick-Ups/TEMP_MATERIALS/M_Gold.M_Gold")
      (elif (== _add_score _blue)
        (`PrimitiveComponent.SetMaterial` (`self.SM_Stud_1`) 0 "/Game/StudentContent/Materials/Pick-Ups/TEMP_MATERIALS/M_Blue.M_Blue")
        (`PrimitiveComponent.SetMaterial` (`self.SM_Stud_2`) 0 "/Game/StudentContent/Materials/Pick-Ups/TEMP_MATERIALS/M_Blue.M_Blue")
        (elif (== _add_score _purple)
          (`PrimitiveComponent.SetMaterial` (`self.SM_Stud_1`) 0 "/Game/StudentContent/Materials/Pick-Ups/TEMP_MATERIALS/M_Purple.M_Purple")
          (`PrimitiveComponent.SetMaterial` (`self.SM_Stud_2`) 0 "/Game/StudentContent/Materials/Pick-Ups/TEMP_MATERIALS/M_Purple.M_Purple"))))))
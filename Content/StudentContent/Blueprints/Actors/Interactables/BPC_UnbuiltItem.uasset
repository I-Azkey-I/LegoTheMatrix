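; Interactable child Blueprint for an unbuilt item that players build by interacting for a set time.
; The first interaction starts a looping one-second countdown timer, which pauses when interaction stops and resumes later, preserving partial progress.
; When time runs out, it asks the game manager to replace it at its transform with a built item, indexed by whether it is a bridge.
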(fn `Decrement Time`
  (bind _time_value (`self.Time Value`))
  ;[0.6795 1 0.5776] Decrement a value for the timer to fire off as a delegate.
  (set `self.Time Value` (- (`self.Time Value`) 1))
  (if (<= _time_value 0)
    ;[0.6795 1 0.5776] Replace the unbuilt item with newly built item.
    (if (`self.IsBridge?`)
      (message `/Game/StudentContent/Blueprints/Libraries/BPI_GameManagement.Replace Item` (`self.Game Manager (Ref)`) self (`self.GetTransform` self) 0)
      (else
        (message `/Game/StudentContent/Blueprints/Libraries/BPI_GameManagement.Replace Item` (`self.Game Manager (Ref)`) self (`self.GetTransform` self) 1)))
    (else
      (`KismetSystemLibrary.PrintString` (`KismetStringLibrary.Conv_IntToString` _time_value)))))

(fn `Interact Effect`
  (params (`Player Character` :type "/Game/StudentContent/Blueprints/Actors/Pawns/Characters/BP_BaseCharacter Object Reference") (`Character Index` :type Integer) (`Is Interacting` :type Boolean))
  ;[0.6795 1 0.5776] Timer for Building Items Mechanic
  (if `Is Interacting`
    (if (`self.Partially Built`)
      (`KismetSystemLibrary.K2_UnPauseTimer` null "Decrement Time")
      (else
        (set `self.Partially Built` true)
        (bind _returnvalue (`KismetSystemLibrary.K2_SetTimer` null "Decrement Time" 1.0 true))
        (set `self.Timer Handle` _returnvalue)))
    (else
      (`KismetSystemLibrary.K2_PauseTimerHandle` (`self.Timer Handle`)))))

(fn `UserConstructionScript`
  (`parent.UserConstructionScript`))
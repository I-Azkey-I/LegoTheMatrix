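; BP_MainCamera is a shared camera actor that follows and frames all active player characters.
; Initiating or updating the player set binds camera updates to each character's OnCharacterMovementUpdated event.
; Each update lerps the focal point mesh toward the players' average location by CameraMovementSpeed.
; It then sets the spring arm length to the largest pairwise player distance, clamped between minimum and maximum camera distances.
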(event `Change Camera Position`
  (params (Players :type "Array of Character Object Reference"))
  ;[0.6795 1 0.5776] Update the camera's position based on the current character's locations in the scene.
  (add `Character.OnCharacterMovementUpdated` Players (delegate `Update Camera`)))

(event `Update Camera`
  (params (DeltaSeconds :type "Float (double-precision)") (OldLocation :type "Vector Structure") (OldVelocity :type "Vector Structure"))
  ;[0.6795 1 0.5776] Update the camera's position based on the current character's locations in the scene.
  (`self.Update Camera Position` (stale `Change Camera Position` Players)))

(fn `Initiate Shared Camera`
  (params (`Spawned Players` :type "Array of Character Object Reference"))
  ;[0.6795 1 0.5776] Call for the shared camera to update it's initial position.
  (bind _output_get (set `self.Spawned Players` `Spawned Players`))
  (`self.Change Camera Position` _output_get))

(fn `Return Min & Max Camera Length`
  (returns (ReturnValue :type "Float (double-precision)"))
  ;[0.6795 1 0.5776] Calculate the minimum and maximum camera length (based on max distance between players).
  (return (`KismetMathLibrary.FClamp` (`.MaxValue` (`KismetMathLibrary.MaxOfFloatArray` (`self.Player Distances`))) (`self.Min Camera Distance`) (`self.Max Camera Distance`))))

(fn `Update Camera Position`
  (params (Players :type "Array of Character Object Reference"))
  ;[0.6795 1 0.5776] Based on the average location of the player(s), set the camera location every tick.
  (bind _output_get (set `self.Active Players` Players))
  (set `self.Previous Camera Location` (`SceneComponent.K2_GetComponentLocation` (`self.SM_FocalPoint`)))
  (bind _returnvalue (`GameplayStatics.GetActorArrayAverageLocation` _output_get))
  (`SceneComponent.K2_SetWorldLocation` (`self.SM_FocalPoint`) (`KismetMathLibrary.VLerp` (`self.Previous Camera Location`) _returnvalue (`self.Camera Movement Speed`)) false false)
  (`self.Update Camera Zoom` (`self.Active Players`)))

(fn `Update Camera Zoom`
  (params (`Active Players` :type "Array of Character Object Reference"))
  ;[1 1 1] Update Camera Distance & Location
  ;;[0.6795 1 0.5776] Calculate the distance between all players & use max. value to determine the min. & max. distance for shared camera.
  (bind _output_get (set `self.Active Players` `Active Players`))
  (for (_array_element _array_index) _output_get
    (set `self.Player` _array_element)
    (for _index (range (+ _array_index 1) (`KismetArrayLibrary.Array_Length` (`self.Active Players`)))
      (`KismetArrayLibrary.Array_Add` (`self.Player Distances`) (`self.GetDistanceTo` (`self.Player`) (`|GetArrayItem` (`self.Active Players`) _index)))))
  ;;[0.6795 1 0.5776] Set the min. & max. distance for shared camera.
  (set `SpringArmComponent.TargetArmLength` (`self.Return Min & Max Camera Length`) (`self.SA_CameraArm`))
  (`KismetArrayLibrary.Array_Clear` (`self.Player Distances`)))

(fn `Update Shared Camera`
  (params (`Updated Players` :type "Array of Character Object Reference"))
  ;[0.6795 1 0.5776] Update the camera's position when player character swaps.
  (bind _output_get (set `self.Updated Players` `Updated Players`))
  (`self.Change Camera Position` _output_get))

(fn `UserConstructionScript`)
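; BP_InteractItem is an interactable world actor with an empty InteractEffect function as the hook for the actual effect.
; BC_Trigger overlaps match the other actor against all BPC_BasePlayer instances and send that player InteractInfo with the item and its in-range state.
; The Interacting event forwards the player, their PlayerIndex and the interaction state to InteractEffect.
; It also caches BP_GameManager on BeginPlay and provides a player-character lookup by index.
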(event `self.ReceiveBeginPlay`
  ;[0.6795 1 0.5776] Find "Game Manager" actor in the scene.
  (bind _returnvalue (`GameplayStatics.GetActorOfClass` "/Game/StudentContent/Blueprints/Managers/BP_GameManager.BP_GameManager_C"))
  (set `self.Game Manager (Ref)` _returnvalue))

(event `self.BC_Trigger.OnComponentBeginOverlap`
  (params (OverlappedComponent :type "PrimitiveComponent Object Reference") (OtherActor :type "Actor Object Reference") (OtherComp :type "PrimitiveComponent Object Reference") (OtherBodyIndex :type Integer) (bFromSweep :type Boolean) (SweepResult :type "HitResult Structure (by ref)"))
  ;[1 1 1] Interacting with Buildable Item
  ;;[0.6795 1 0.5776] If player is in range of the overlapping trigger, allow them to interact.
  (bind _outactors (`GameplayStatics.GetAllActorsOfClass` "/Game/StudentContent/Blueprints/Actors/Pawns/Characters/Players/BPC_BasePlayer.BPC_BasePlayer_C"))
  (bind _output_get (set `self.Base Players Array (Ref)` _outactors))
  (for _array_element _output_get
    (if (== _array_element OtherActor)
      (bind _output_get_2 (set `self.Player in Range` true))
      (`/Game/StudentContent/Blueprints/Actors/Pawns/Characters/Players/BPC_BasePlayer.Interact Info` _array_element self _output_get_2))))

(event `self.BC_Trigger.OnComponentEndOverlap`
  (params (OverlappedComponent :type "PrimitiveComponent Object Reference") (OtherActor :type "Actor Object Reference") (OtherComp :type "PrimitiveComponent Object Reference") (OtherBodyIndex :type Integer))
  ;[1 1 1] Interacting with Buildable Item
  ;;[0.6795 1 0.5776] If player is out of range of the overlapping trigger, stop them from interacting.
  (bind _outactors (`GameplayStatics.GetAllActorsOfClass` "/Game/StudentContent/Blueprints/Actors/Pawns/Characters/Players/BPC_BasePlayer.BPC_BasePlayer_C"))
  (bind _output_get (set `self.Base Players Array (Ref)` _outactors))
  (for _array_element _output_get
    (if (== _array_element OtherActor)
      (bind _output_get_2 (set `self.Player in Range` false))
      (`/Game/StudentContent/Blueprints/Actors/Pawns/Characters/Players/BPC_BasePlayer.Interact Info` _array_element self _output_get_2))))

(event `/Game/StudentContent/Blueprints/Libraries/BPI_Interactions.Interacting`
  (params (`Player Character` :type "/Game/StudentContent/Blueprints/Actors/Pawns/Characters/Players/BPC_BasePlayer Object Reference") (Interacting :type Boolean))
  ;[1 1 1] Interacting with Buildable Item
  ;;[0.6795 1 0.5776] Apply the interaction effect to this actor.
  (`self.Interact Effect` `Player Character` (`/Game/StudentContent/Blueprints/Actors/Pawns/Characters/Players/BPC_BasePlayer.Player Index` `Player Character`) Interacting))

(fn `Interact Effect`
  (params (`Player Character` :type "/Game/StudentContent/Blueprints/Actors/Pawns/Characters/BP_BaseCharacter Object Reference") (`Character Index` :type Integer) (`Is Interacting` :type Boolean))
  ;[0.6795 1 0.5776] Apply the base interaction effect.
)

(fn `Retrieve Player Character`
  (params (Index :type Integer))
  (returns (ReturnValue :type "Character Object Reference"))
  ;[0.6795 1 0.5776] Return the player character that's interacting.
  (return (`GameplayStatics.GetPlayerCharacter` (`GameplayStatics.GetPlayerControllerID` (`GameplayStatics.GetPlayerController` Index)))))

(fn `UserConstructionScript`)
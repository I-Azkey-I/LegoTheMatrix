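; Game manager for local multiplayer with a shared camera, handling player creation, character spawning and swapping, and game start.
; SpawnInputRecievers creates a local player and possessed input-receiver pawn per BP_PlayerSpawn, but its setup chain is disconnected from the empty BeginPlay.
; SpawnPlayer spawns and possesses an indexed character at its receiver's transform, viewed through BP_MainCamera.
; StartGame sets HasGameStarted once enough players have spawned and initiates the shared camera on them.
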(event `self.ReceiveBeginPlay`
  ;[1 1 1] Initialisation (Game Starting Events)
)

(fn `Decrement Time`)

(fn `Get Player Spawn Locals`
  ;[0.6795 1 0.5776] Find all player start locations in the scene.
  (bind _outactors (`GameplayStatics.GetAllActorsOfClass` "/Game/StudentContent/Blueprints/Actors/BP_PlayerSpawn.BP_PlayerSpawn_C"))
  (set `self.Player Spawn Locals` _outactors)
  (return))

(fn `Is In Play State?`
  (returns (`In Play State` :type Boolean))
  ;[0.6795 1 0.5776] Return the current game state.
  (return (`self.Has Game Started?`)))

(fn `Name to Int`
  (params (`Player Start` :type "PlayerStart Object Reference"))
  (returns (`Index Value` :type Integer))
  (return (`KismetStringLibrary.Conv_StringToInt` (`KismetStringLibrary.Conv_NameToString` (`PlayerStart.PlayerStartTag` `Player Start`)))))

(fn `Remove Unused Cameras`
  ;[0.6795 1 0.5776] Destroy all controller cameras possessing players.
  (bind _outactors (`GameplayStatics.GetAllActorsOfClass` "/Script/Engine.CameraActor"))
  (for _array_element _outactors
    (`self.K2_DestroyActor` _array_element)
    (return)))

(fn `Return Spawn Transform`
  (returns (ReturnValue :type "Transform Structure (by ref)"))
  (bind _player_spawn_locals (`self.Player Spawn Locals`))
  ;[0.6795 1 0.5776] Return the transform data of each player start location.
  (return (`self.GetTransform` (`|GetArrayItem` _player_spawn_locals (`KismetMathLibrary.RandomIntegerInRange` 0 (- (`KismetArrayLibrary.Array_Length` _player_spawn_locals) 1))))))

(fn `Spawn Input Recievers`
  (locals (`Input Reciever Index (L)` :type Integer))
  (bind _player_controllers (`self.Player Controllers`))
  ;[1 1 1] Input Receiver Management
  ;;[0.6795 1 0.5776] Store the index & element of each input receiever.
  (for (_array_element _array_index) (`self.Player Spawn Locals`)
    (bind _output_get (set `local.Input Reciever Index (L)` _array_index))
    ;;[0.6795 1 0.5776] Create a player ready for possession by controllers.
    (bind _output_get_2 (set `/Game/StudentContent/Blueprints/Actors/BP_PlayerSpawn.PlayerSpawnID` _output_get _array_element))
    (if (== _output_get_2 _output_get)
      (`GameplayStatics.CreatePlayer` -1)
      ;;[0.6795 1 0.5776] Spawn an input receiver pawn per player that's created.
      (bind _returnvalue (`|SpawnActorFromClass` "/Game/StudentContent/Blueprints/Actors/Pawns/BP_InputReceiver.BP_InputReceiver_C" (`self.GetTransform` (`|GetArrayItem` (`self.Player Spawn Locals`) (`local.Input Reciever Index (L)`))) "Undefined" "OverrideRootScale" null (`local.Input Reciever Index (L)`) null))
      (`KismetArrayLibrary.Array_AddUnique` (`self.Input Receievers`) _returnvalue)
      ;;[0.6795 1 0.5776] Possess each input receiver with the relevant player controller.
      (`Controller.Possess` (`GameplayStatics.GetPlayerController` (`local.Input Reciever Index (L)`)) _returnvalue)
      (bind _returnvalue_2 (`KismetArrayLibrary.Array_AddUnique` _player_controllers (`GameplayStatics.GetPlayerController` (`local.Input Reciever Index (L)`))))
      ;;[0.6795 1 0.5776] Initialise the player controllers for each input receiver.
      (message `/Game/StudentContent/Blueprints/Libraries/BPI_StartGame.Initialise Controller` (`|GetArrayItem` _player_controllers _returnvalue_2))
      ;;[0.6795 1 0.5776] Set the default camera to the main shared camera.
      (`PlayerController.SetViewTargetWithBlend` (`GameplayStatics.GetPlayerController` (`local.Input Reciever Index (L)`)) (`self.Main Camera`) 0.0 "VTBlend_Linear" 0.0 false)
      (for _array_element_2 (`self.Input Receievers`)
        (`KismetSystemLibrary.PrintString` (`KismetSystemLibrary.GetDisplayName` _array_element_2))
        (return))))
  ;;[0.6795 1 0.5776] Once all players have spawned, remove the controller cameras.
  (`self.Remove Unused Cameras`))

(fn `Spawn Player`
  (params (`Current Player Index` :type Integer) (`Input Receiver` :type "/Game/StudentContent/Blueprints/Actors/Pawns/BP_InputReceiver Object Reference"))
  (returns (Return :type Boolean))
  (locals (`Input Receiver (L)` :type "/Game/StudentContent/Blueprints/Actors/Pawns/BP_InputReceiver Object Reference"))
  ;[0.6795 1 0.5776] Store parameters as variables (some local).
  (bind _output_get (set `self.Current Player Index` `Current Player Index`))
  (set `local.Input Receiver (L)` `Input Receiver`)
  ;[0.6795 1 0.5776] Spawn a player character into the scene at the relevant spawn location.
  (bind _player_character (`self.Spawn Player Character` _output_get (`self.GetTransform` (`local.Input Receiver (L)`))))
  (`KismetArrayLibrary.Array_Add` (`self.Spawned Players`) _player_character)
  ;[0.6795 1 0.5776] Possess the newly spawned character & set it's controller camera to be the main shared camera.
  (`Controller.Possess` (`GameplayStatics.GetPlayerController` (`self.Current Player Index`)) _player_character)
  (`PlayerController.SetViewTargetWithBlend` (`GameplayStatics.GetPlayerController` (`self.Current Player Index`)) (`self.Main Camera`) 0.0 "VTBlend_Linear" 0.0 false)
  (return false))

(fn `Spawn Player Character`
  (params (`Player Index` :type Integer) (`Player Transform` :type "Transform Structure (by ref)"))
  (returns (`Player Character` :type "/Game/StudentContent/Blueprints/Actors/Pawns/Characters/BP_BasePlayer Object Reference"))
  (bind _output (`|GetArrayItem` (`self.Characters`) `Player Index`))
  ;[0.6795 1 0.5776] Spawn a player character (based on character's array) at relevant location.
  (bind _returnvalue (`|SpawnActorFromClass` (select `int` `Player Index` :`0` _output :`1` _output) (`KismetMathLibrary.MakeTransform` (.location `Player Transform`) (struct) (.scale `Player Transform`)) "Undefined" "OverrideRootScale" null `Player Index` null))
  (return _returnvalue))

(fn `Start Game`
  (returns (Return :type Boolean))
  ;[1 1 1] Initial "Start Game" Behaviour
  ;;[0.6795 1 0.5776] Begin the game when min. number of players has been reached.
  (if (>= (`KismetArrayLibrary.Array_Length` (`self.Spawned Players`)) (`self.Min Number of Players`))
    (set `self.Has Game Started?` true)
    ;;[0.6795 1 0.5776] Instantiate the shared camera for all readied players.
    (`/Game/StudentContent/Blueprints/Actors/Cameras/BP_MainCamera.Initiate Shared Camera` (`self.Main Camera`) (`self.Spawned Players`))
    (return false)))

(fn `Swap Character`
  (params (`Character Index` :type Integer) (`Transform Data` :type "Transform Structure"))
  (returns (`New Player Character` :type "/Game/StudentContent/Blueprints/Actors/Pawns/Characters/BP_BaseCharacter Object Reference") (Return :type Boolean))
  ;[0.6795 1 0.5776] Swap the current character with a new one.
  (bind _player_character (`self.Spawn Player Character` `Character Index` `Transform Data`))
  (return _player_character false))

(fn `UserConstructionScript`)